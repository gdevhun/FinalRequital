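; Prototype fire hydrant trap that toggles its particle effect on and off on a looping three-second timer.
; While active, a second timer calls ApplyDamage at each Interval, but the ApplyDamageEffect event it triggers is empty.
; Disconnected logic tracks overlapping characters and applies separate GAS effects to players and monsters, plus a hit ability on players.
; As wired, none of that logic runs, so this graph deals no damage.
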(event Custom|ApplyDamageEffect)

(event Custom|ToggleTrapActive
  (bind _output_get (Variables|Default|SetbIsTrapActive (not (Variables|Default|GetbIsTrapActive))))
  (if _output_get
    (Components|Activation|Activate (Variables|Default|GetParticleSystem) false)
    (bind _returnvalue (Utilities|Time|SetTimerbyEvent (delegate Custom|ApplyDamage) (Variables|Default|GetInterval) true))
    (else
      (Components|Activation|Deactivate (Variables|Default|GetParticleSystem))
      (Utilities|Time|ClearandInvalidateTimerbyHandle _returnvalue))))

(event Custom|ApplyDamage
  (CallFunction|ApplyDamageEffect))

(event EventBeginPlay
  (Variables|Default|SetbIsTrapActive false)
  (Components|Activation|Deactivate (Variables|Default|GetParticleSystem))
  (Utilities|Time|SetTimerbyEvent (delegate Custom|ToggleTrapActive) 3.0 true))

(fn ConstructionScript)