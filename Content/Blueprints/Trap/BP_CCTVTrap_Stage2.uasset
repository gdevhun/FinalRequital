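; CCTV trap for Stage 2 that sweeps its spotlight in pitch between MinPitch and MaxPitch.
; On BeginPlay it binds to the initialize and start gimmick events of BP_Stage2GimmickManager and caches its starting transform.
; Activation plays one of five fixed-length timelines, picked by TrapIntervalType, to lerp the light's rotation.
; Deactivation stops that timeline and restores the actor's initial transform.
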(event Custom|DeactivateTrap
  (CallFunction|InitializeTransform)
  (switch Utilities|FlowControl|Switch|SwitchonETrapIntervalType (Variables|Default|GetTrapIntervalType)
    (:Interval_1_25
      (bind _float (Timeline|RotTimeline_1_25sec Stop)
        (:Update
          (Transformation|SetRelativeRotation (Variables|Default|GetSpotLight) (Math|Rotator|Lerp(Rotator) (Math|Rotator|MakeRotator 0.0 (Variables|Default|GetMaxPitch) 0.0) (Math|Rotator|MakeRotator 0.0 (Variables|Default|GetMinPitch) 0.0) _float) false false))))
    (:Interval_1_5
      (bind _float_2 (Timeline|RotTimeline_1_5sec Stop)
        (:Update
          (Transformation|SetRelativeRotation (Variables|Default|GetSpotLight) (Math|Rotator|Lerp(Rotator) (Math|Rotator|MakeRotator 0.0 (Variables|Default|GetMaxPitch) 0.0) (Math|Rotator|MakeRotator 0.0 (Variables|Default|GetMinPitch) 0.0) _float_2) false false))))
    (:Interval_2
      (bind _float_3 (Timeline|RotTimeline_2sec Stop)
        (:Update
          (Transformation|SetRelativeRotation (Variables|Default|GetSpotLight) (Math|Rotator|Lerp(Rotator) (Math|Rotator|MakeRotator 0.0 (Variables|Default|GetMaxPitch) 0.0) (Math|Rotator|MakeRotator 0.0 (Variables|Default|GetMinPitch) 0.0) _float_3) false false))))
    (:Interval_2_5
      (bind _float_4 (Timeline|RotTimeline_2_5sec Stop)
        (:Update
          (Transformation|SetRelativeRotation (Variables|Default|GetSpotLight) (Math|Rotator|Lerp(Rotator) (Math|Rotator|MakeRotator 0.0 (Variables|Default|GetMaxPitch) 0.0) (Math|Rotator|MakeRotator 0.0 (Variables|Default|GetMinPitch) 0.0) _float_4) false false))))
    (:Interval_3
      (bind _float_5 (Timeline|RotTimeline_3sec Stop)
        (:Update
          (Transformation|SetRelativeRotation (Variables|Default|GetSpotLight) (Math|Rotator|Lerp(Rotator) (Math|Rotator|MakeRotator 0.0 (Variables|Default|GetMaxPitch) 0.0) (Math|Rotator|MakeRotator 0.0 (Variables|Default|GetMinPitch) 0.0) _float_5) false false))))))

(event Custom|InitializeTransform
  (Transformation|SetActorTransform (Variables|Default|GetInitTransform)))

(event Custom|ActivateTrap
  (switch Utilities|FlowControl|Switch|SwitchonETrapIntervalType (Variables|Default|GetTrapIntervalType)
    (:Interval_1_25
      (bind _float (Timeline|RotTimeline_1_25sec PlayFromStart)
        (:Update
          (Transformation|SetRelativeRotation (Variables|Default|GetSpotLight) (Math|Rotator|Lerp(Rotator) (Math|Rotator|MakeRotator 0.0 (Variables|Default|GetMaxPitch) 0.0) (Math|Rotator|MakeRotator 0.0 (Variables|Default|GetMinPitch) 0.0) _float) false false))))
    (:Interval_1_5
      (bind _float_2 (Timeline|RotTimeline_1_5sec PlayFromStart)
        (:Update
          (Transformation|SetRelativeRotation (Variables|Default|GetSpotLight) (Math|Rotator|Lerp(Rotator) (Math|Rotator|MakeRotator 0.0 (Variables|Default|GetMaxPitch) 0.0) (Math|Rotator|MakeRotator 0.0 (Variables|Default|GetMinPitch) 0.0) _float_2) false false))))
    (:Interval_2
      (bind _float_3 (Timeline|RotTimeline_2sec PlayFromStart)
        (:Update
          (Transformation|SetRelativeRotation (Variables|Default|GetSpotLight) (Math|Rotator|Lerp(Rotator) (Math|Rotator|MakeRotator 0.0 (Variables|Default|GetMaxPitch) 0.0) (Math|Rotator|MakeRotator 0.0 (Variables|Default|GetMinPitch) 0.0) _float_3) false false))))
    (:Interval_2_5
      (bind _float_4 (Timeline|RotTimeline_2_5sec PlayFromStart)
        (:Update
          (Transformation|SetRelativeRotation (Variables|Default|GetSpotLight) (Math|Rotator|Lerp(Rotator) (Math|Rotator|MakeRotator 0.0 (Variables|Default|GetMaxPitch) 0.0) (Math|Rotator|MakeRotator 0.0 (Variables|Default|GetMinPitch) 0.0) _float_4) false false))))
    (:Interval_3
      (bind _float_5 (Timeline|RotTimeline_3sec PlayFromStart)
        (:Update
          (Transformation|SetRelativeRotation (Variables|Default|GetSpotLight) (Math|Rotator|Lerp(Rotator) (Math|Rotator|MakeRotator 0.0 (Variables|Default|GetMaxPitch) 0.0) (Math|Rotator|MakeRotator 0.0 (Variables|Default|GetMinPitch) 0.0) _float_5) false false))))))

(event EventBeginPlay
  (bind _returnvalue (Actor|GetActorOfClass "/Game/Blueprints/Stage2/BP_Stage2GimmickManager.BP_Stage2GimmickManager_C"))
  (EventDispatchers|BindEventtoInitializeGimmick _returnvalue (EventDispatchers|CreateEvent :!event Custom|DeactivateTrap))
  (EventDispatchers|BindEventtoStartGimmick _returnvalue (EventDispatchers|CreateEvent :!event Custom|ActivateTrap))
  (Variables|Default|SetInitTransform (Transformation|GetActorTransform)))

(fn ConstructionScript)