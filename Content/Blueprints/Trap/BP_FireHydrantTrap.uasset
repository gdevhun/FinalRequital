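; Fire hydrant trap that cycles on and off on a fixed looping timer, damaging characters inside its collision box while active.
; The toggle switches the particle system and starts or clears a repeating damage timer, while box overlaps maintain the list of affected characters.
; Damage uses GAS effects: players receive the Lv2 effect and trigger a hit-reaction ability, while other characters receive the Lv1 effect.
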(event OnComponentBeginOverlap(CollisionBox)
  (params (OverlappedComponent :type Primitive%20Component%20Object%20Reference) (OtherActor :type Actor%20Object%20Reference) (OtherComp :type Primitive%20Component%20Object%20Reference) (OtherBodyIndex :type Integer) (bFromSweep :type Boolean) (SweepResult :type Hit%20Result%20Structure%20%28by%20ref%29))
  (bind _ascharacter (Utilities|Casting|CastToCharacter OtherActor))
  (Utilities|Array|AddUnique (Variables|Default|GetOverlappingChar) _ascharacter))

(event OnComponentEndOverlap(CollisionBox)
  (params (OverlappedComponent :type Primitive%20Component%20Object%20Reference) (OtherActor :type Actor%20Object%20Reference) (OtherComp :type Primitive%20Component%20Object%20Reference) (OtherBodyIndex :type Integer))
  (bind _ascharacter (Utilities|Casting|CastToCharacter OtherActor))
  (Utilities|Array|RemoveItem (Variables|Default|GetOverlappingChar) _ascharacter))

(event Custom|ApplyDamageEffect
  (bind _returnvalue (Ability|GetAbilitySystemComponent 0))
  (for _array_element (Variables|Default|GetOverlappingChar)
    (Utilities|Casting|CastToFRGASCharacterPlayer _array_element
      (:then
        (GameplayEffects|ApplyGameplayEffectSpecToTarget _returnvalue (GameplayEffects|MakeOutgoingSpec :self (Variables|Default|GetASC) :GameplayEffectClass "/Game/Blueprints/GE/Trap/BPGE_HydrantTrap_Lv2.BPGE_HydrantTrap_Lv2_C") (Ability|GetAbilitySystemComponent _array_element))
        (Abilities|TryActivateAbilitybyClass (Ability|GetAbilitySystemComponent _array_element) "/Game/Blueprints/GA/BPGA_PlayerHit.BPGA_PlayerHit_C" true))
      (:CastFailed
        (GameplayEffects|ApplyGameplayEffectSpecToTarget _returnvalue (GameplayEffects|MakeOutgoingSpec :self (Variables|Default|GetASC) :GameplayEffectClass "/Game/Blueprints/GE/Trap/BPGE_HydrantTrap_Lv1.BPGE_HydrantTrap_Lv1_C") (Ability|GetAbilitySystemComponent _array_element))))))

(event Custom|ToggleTrapActive
  (bind _output_get (Variables|Default|SetbIsTrapActive (not (Variables|Default|GetbIsTrapActive))))
  (if _output_get
    (Components|Activation|Activate (Variables|Default|GetParticleSystem) false)
    (bind _returnvalue (Utilities|Time|SetTimerbyEvent (delegate Custom|ApplyDamage) (Variables|Default|GetInterval) true))
    (else
      (Components|Activation|Deactivate (Variables|Default|GetParticleSystem))
      (Utilities|Time|ClearandInvalidateTimerbyHandle _returnvalue))))

(event Custom|ApplyDamage
  (CallFunction|ApplyDamageEffect))

(event EventBeginPlay
  (Variables|Default|SetbIsTrapActive false)
  (Components|Activation|Deactivate (Variables|Default|GetParticleSystem))
  (Utilities|Time|SetTimerbyEvent (delegate Custom|ToggleTrapActive) 3.0 true))

(fn ConstructionScript)