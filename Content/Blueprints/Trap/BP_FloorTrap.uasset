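; BP_FloorTrap is a floor trap actor that animates its TrapMesh vertically between a lowered and a raised position.
; BeginPlay waits StartDelay, then calls ActivateTrap, which switches on TrapIntervalType to play one of five fixed-interval timelines from the start.
; Each timeline's float track drives a lerp on the mesh's relative Z, so timing comes from the chosen timeline rather than a computed play rate.
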(event Custom|ActivateTrap
  ;[1 1 1] TrapActiveInterval 이 소숫점에만 정확히 맞춰야함.
  (switch Utilities|FlowControl|Switch|SwitchonETrapIntervalType (Variables|Default|GetTrapIntervalType)
    (:Interval_1_25
      (bind _floatz (Timeline|Timeline_1_25sec PlayFromStart)
        (:Update
          (Transformation|SetRelativeLocation (Variables|Default|GetTrapMesh) (Math|Vector|MakeVector 0.0 0.0 (.z (Math|Vector|Lerp(Vector) (Math|Vector|MakeVector 0.0 0.0 -1.4e+02) (Math|Vector|MakeVector 0.0 0.0 -4e+01) _floatz))) false false))))
    (:Interval_1_5
      (bind _floatz_2 (Timeline|Timeline_1_5sec PlayFromStart)
        (:Update
          (Transformation|SetRelativeLocation (Variables|Default|GetTrapMesh) (Math|Vector|MakeVector 0.0 0.0 (.z (Math|Vector|Lerp(Vector) (Math|Vector|MakeVector 0.0 0.0 -1.4e+02) (Math|Vector|MakeVector 0.0 0.0 -4e+01) _floatz_2))) false false))))
    (:Interval_2
      (bind _floatz_3 (Timeline|Timeline_2sec PlayFromStart)
        (:Update
          (Transformation|SetRelativeLocation (Variables|Default|GetTrapMesh) (Math|Vector|MakeVector 0.0 0.0 (.z (Math|Vector|Lerp(Vector) (Math|Vector|MakeVector 0.0 0.0 -1.4e+02) (Math|Vector|MakeVector 0.0 0.0 -4e+01) _floatz_3))) false false))))
    (:Interval_2_5
      (bind _floatz_4 (Timeline|Timeline_2_5sec PlayFromStart)
        (:Update
          (Transformation|SetRelativeLocation (Variables|Default|GetTrapMesh) (Math|Vector|MakeVector 0.0 0.0 (.z (Math|Vector|Lerp(Vector) (Math|Vector|MakeVector 0.0 0.0 -1.4e+02) (Math|Vector|MakeVector 0.0 0.0 -4e+01) _floatz_4))) false false))))
    (:Interval_3
      (bind _floatz_5 (Timeline|Timeline_3_0sec PlayFromStart)
        (:Update
          (Transformation|SetRelativeLocation (Variables|Default|GetTrapMesh) (Math|Vector|MakeVector 0.0 0.0 (.z (Math|Vector|Lerp(Vector) (Math|Vector|MakeVector 0.0 0.0 -1.4e+02) (Math|Vector|MakeVector 0.0 0.0 -4e+01) _floatz_5))) false false))))))

(event EventBeginPlay
  (Utilities|FlowControl|Delay (Variables|Default|GetStartDelay))
  (CallFunction|ActivateTrap))

(fn ConstructionScript)