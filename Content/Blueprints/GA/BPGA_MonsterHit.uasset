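; Gameplay ability that plays a monster's hit reaction, freezing the avatar's movement for its duration.
; Activation commits the ability or ends it on failure; the commit event plays the AM_Hit montage and sets character movement mode to None.
; Montage completion, blend out, interruption or cancellation ends the ability, and OnEndAbility restores Walking mode.
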(event Ability|EventOnEndAbility
  (params (bWasCancelled :type Boolean))
  (bind _ascharacter (Utilities|Casting|CastToCharacter (Ability|GetAvatarActorfromActorInfo)))
  (Pawn|Components|CharacterMovement|SetMovementMode (Variables|/Script/Engine.Character|GetCharacterMovement _ascharacter) "MOVE_Walking" 0))

(event Ability|EventCommitExecute
  (|PlayMontageandWaitProxy "None" "/Game/Animations/Montages/AM_Hit.AM_Hit" 1.0 "None" true 1.0 0.0 false
    (:then
      (bind _ascharacter (Utilities|Casting|CastToCharacter (Ability|GetAvatarActorfromActorInfo)))
      (Pawn|Components|CharacterMovement|SetMovementMode (Variables|/Script/Engine.Character|GetCharacterMovement _ascharacter) "MOVE_None" 0))
    (:OnCompleted
      (Ability|EndAbility :!label _label))
    (:OnBlendOut
      (goto _label))
    (:OnInterrupted
      (goto _label))
    (:OnCancelled
      (goto _label))))

(event Ability|EventActivateAbility
  (bind _returnvalue (Ability|CommitAbility))
  (if (not _returnvalue)
    (Ability|EndAbility)))