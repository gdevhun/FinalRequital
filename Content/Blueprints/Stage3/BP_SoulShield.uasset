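; BP_SoulShield is a Stage 3 actor with Ability System health whose depletion fails the run, pausing the game and showing the retry menu.
; ApplyResetHp restores health by applying the SoulShield heal GameplayEffect to its own ASC.
; A separate Destroy event plays an electric burst, activates two Niagara effects and staggered sounds, then removes the actor after a short delay.
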(event Custom|ApplyResetHp
  (GameplayEffects|ApplyGameplayEffectToSelf :self (Variables|Default|GetASC) :GameplayEffectClass "/Game/Blueprints/GE/BPGE_SoulShieldHeal.BPGE_SoulShieldHeal_C"))

(event Custom|Destroy
  (Effects|SpawnEmitteratLocation "/Game/Realistic_Starter_VFX_Pack_Vol2/Particles/Destruction/P_Destruction_Electric.P_Destruction_Electric" (Transformation|GetActorLocation) "0, 0, 0" "5.000000,5.000000,5.000000")
  (Components|Activation|Activate (Variables|Default|GetNiagara) true)
  (Utilities|FlowControl|Sequence
    (:then_0
      (Audio|PlaySound2D "/Game/Audio/SFX/Player/ground-smash-cast.ground-smash-cast" 1.0 1.0 0.0 0 0)
      (Utilities|FlowControl|Delay 0.3)
      (Audio|PlaySound2D "/Game/Audio/SFX/Player/SFX_Telpo.SFX_Telpo" 1.0 1.0 0.0 0 0))
    (:then_1
      (Utilities|FlowControl|Delay 3.0)
      (Actor|DestroyActor))))

(event EventBeginPlay)

(event EventOnOutOfHealth
  (Game|SetGamePaused true)
  (bind _returnvalue (UserInterface|CreateWidget "/Game/UI/MainMenu/WBP_RetryMenu.WBP_RetryMenu_C"))
  (UserInterface|Viewport|AddtoViewport _returnvalue 0))

(fn ConstructionScript)