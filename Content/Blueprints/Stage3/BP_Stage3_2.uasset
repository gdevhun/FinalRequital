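; Stage 3 interactable that opens a dialogue and, once it finishes, launches a timed survival encounter around the Soul Shield.
; The finish callback resets the shield's HP immediately while a Delay chain shows the notify text, then a preparation timer widget whose RemainingTime sets the wait.
; Afterwards it binds a shield HP widget to BP_SoulShield, starts every BP_MonsterSpawner and shows the survival timer.
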(event EventBeginPlay)

(event EventInteract
  (|CallParentFunction)
  (Class|FRDialogueActor|StartDialogue))

(event EventDialogueFinishCallback
  (Utilities|FlowControl|Sequence
    (:then_0
      (Utilities|FlowControl|Delay 0.5)
      (bind _returnvalue (UserInterface|CreateWidget "/Game/UI/StagePlay/WBP_Stage3NotifyText.WBP_Stage3NotifyText_C"))
      (UserInterface|Viewport|AddtoViewport _returnvalue 0)
      (Utilities|FlowControl|Delay 5.0)
      ;[1 1 1] 이 위젯에서 스테이지 준비시간 설정
      (bind _returnvalue_2 (UserInterface|CreateWidget "/Game/UI/StagePlay/WBP_Stage3PrepareTimer.WBP_Stage3PrepareTimer_C" (Game|GetPlayerController 0)))
      (UserInterface|Viewport|AddtoViewport _returnvalue_2 0)
      (Utilities|FlowControl|Delay (Variables|/Game/UI/StagePlay/WBP_Stage3PrepareTimer.WBP_Stage3PrepareTimer_C|GetRemainingTime _returnvalue_2))
      (Utilities|FlowControl|Sequence
        (:then_0
          (bind _returnvalue_3 (UserInterface|CreateWidget "/Game/UI/StagePlay/WBP_SoulShieldHp.WBP_SoulShieldHp_C" (Game|GetPlayerController 0)))
          (bind _returnvalue_4 (Actor|GetActorOfClass "/Game/Blueprints/Stage3/BP_SoulShield.BP_SoulShield_C"))
          (Class|FRUserWidget|SetAbilitySystemComponent _returnvalue_3 _returnvalue_4)
          (UserInterface|Viewport|AddtoViewport _returnvalue_3 0)
          (bind _outactors (Actor|GetAllActorsOfClass "/Game/Blueprints/Stage3/BP_MonsterSpawner.BP_MonsterSpawner_C"))
          (for _array_element _outactors
            (Class|FRMonsterSpawner|StartSpawn _array_element)))
        (:then_1
          ;[1 1 1] 스테이지 버터야하는 시간
          (bind _returnvalue_5 (UserInterface|CreateWidget "/Game/UI/StagePlay/WBP_Stage3Timer.WBP_Stage3Timer_C" (Game|GetPlayerController 0)))
          (UserInterface|Viewport|AddtoViewport _returnvalue_5 0))))
    (:then_1
      (bind _returnvalue_6 (Actor|GetActorOfClass "/Game/Blueprints/Stage3/BP_SoulShield.BP_SoulShield_C"))
      (Default|ApplyResetHp _returnvalue_6))))

(fn ConstructionScript)