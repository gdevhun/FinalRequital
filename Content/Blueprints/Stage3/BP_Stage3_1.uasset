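; BP_Stage3_1 is a Stage 3 interactable that starts a dialogue, then stages the tutorial monster's appearance.
; When the dialogue finishes, it plays the Stage3_Tutorial level sequence alongside a delay-timed chain on BP_S3Monster_Tuto.
; That chain finds the monster by class, spawns its emitter, unhides its mesh, sets its move mode, then moves it to a hard-coded world location.
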(event EventBeginPlay)

(event EventInteract
  (|CallParentFunction)
  (Class|FRDialogueActor|StartDialogue))

(event EventDialogueFinishCallback
  (Utilities|FlowControl|Sequence
    (:then_0
      ;[1 1 1] 시퀀스 후 기억영상
      (bind _outactor (Sequencer|Player|CreateLevelSequencePlayer "/Game/Cinematic/Stage3_Tutorial.Stage3_Tutorial"))
      (Sequencer|Player|Play (Variables|/Script/LevelSequence.LevelSequenceActor|GetSequencePlayer _outactor) :!class /Script/MovieScene.MovieSceneSequencePlayer))
    (:then_1
      (Utilities|FlowControl|Delay 1.0)
      (bind _returnvalue (Actor|GetActorOfClass "/Game/Blueprints/Characters/Stage3/BP_S3Monster_Tuto.BP_S3Monster_Tuto_C"))
      (Default|SpawnEmitter _returnvalue)
      (Utilities|FlowControl|Delay 1.0)
      (Development|SetHiddeninGame (Variables|/Script/Engine.Character|GetMesh _returnvalue) false false)
      (Default|SetMoveMode _returnvalue)
      (Utilities|FlowControl|Delay 2.0)
      (Transformation|SetActorLocation _returnvalue "-5763.000000,466.000000,2672.000000" false false))))

(fn ConstructionScript)