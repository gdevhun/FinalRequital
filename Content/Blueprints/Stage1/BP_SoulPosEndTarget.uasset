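; End target for the Stage 1 soul dribble challenge, handling its success cleanup and stage-clear sequence.
; When BP_Soul enters the Box, it destroys the soul and every actor tagged StageFinishDestoyActor.
; A separate PlayLevelSequence event, not called within this Blueprint, fades the screen and plays Stage1_Clear with player input disabled.
; After timed delays it restores input, fades again and activates BP_LevelPortal.
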(event OnComponentBeginOverlap(Box)
  (params (OverlappedComponent :type Primitive%20Component%20Object%20Reference) (OtherActor :type Actor%20Object%20Reference) (OtherComp :type Primitive%20Component%20Object%20Reference) (OtherBodyIndex :type Integer) (bFromSweep :type Boolean) (SweepResult :type Hit%20Result%20Structure%20%28by%20ref%29))
  ;[1 1 1] 드리블 성공시 영혼, 데스크 엑터 destroy
  (bind _asbp_soul (Utilities|Casting|CastToBP_Soul OtherActor))
  (Actor|DestroyActor _asbp_soul)
  (bind _outactors (Actor|GetAllActorswithTag "StageFinishDestoyActor"))
  (for _array_element _outactors
    (Actor|DestroyActor _array_element)))

(event Custom|PlayLevelSequence
  (bind _fadewidget (Variables|Default|GetFadeWidget))
  (bind _fadewidget_2 (Variables|Default|GetFadeWidget))
  (UserInterface|Viewport|AddtoViewport _fadewidget 0)
  (Default|PlayFadeOut _fadewidget)
  (Input|DisableInput (Game|GetPlayerCharacter 0) (Game|GetPlayerController 0))
  ;[1 1 1] 여기에 영혼드리블을 다 성공했을 때 호출할 레벨시퀀스 지정
  (bind _outactor (Sequencer|Player|CreateLevelSequencePlayer "/Game/Cinematic/Stage1_Clear.Stage1_Clear"))
  (Sequencer|Player|Play (Variables|/Script/LevelSequence.LevelSequenceActor|GetSequencePlayer _outactor) :!class /Script/MovieScene.MovieSceneSequencePlayer)
  (Utilities|FlowControl|Delay 5.0)
  (Input|EnableInput (Game|GetPlayerCharacter 0) (Game|GetPlayerController 0))
  (UserInterface|Viewport|AddtoViewport _fadewidget_2 0)
  (Default|PlayFadeOut _fadewidget_2)
  (Utilities|FlowControl|Delay 0.5)
  (bind _returnvalue (Actor|GetActorOfClass "/Game/Blueprints/Interactive/BP_LevelPortal.BP_LevelPortal_C"))
  (Class|FRLevelPortal|ActivatePortal _returnvalue))

(event EventBeginPlay)

(fn ConstructionScript)