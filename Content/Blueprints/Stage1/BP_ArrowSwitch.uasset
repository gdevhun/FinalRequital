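; Stage 1 arrow switch that swings open a door when shot and plays a one-time introductory cutscene.
; The first BP_ArrowProjectile hit on the switch mesh triggers a timeline-driven door rotation and an opening sound.
; The first character overlap with the box disables input, plays a zoom-in Level Sequence, then after delays relocates this actor, restores input and triggers interaction with the BP_Stage1_4 actor.
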(event OnComponentHit(SM_ArrowSwitch)
  (params (HitComponent :type Primitive%20Component%20Object%20Reference) (OtherActor :type Actor%20Object%20Reference) (OtherComp :type Primitive%20Component%20Object%20Reference) (NormalImpulse :type Vector :default "0, 0, 0") (Hit :type Hit%20Result%20Structure%20%28by%20ref%29))
  (if (Class|GameplayStatics|ObjectIsA OtherActor "/Game/Blueprints/Weapon/BP_ArrowProjectile.BP_ArrowProjectile_C")
    (Utilities|FlowControl|DoOnce false
      (:Completed
        (CallFunction|ActivateRotatingDoor)
        (Audio|PlaySound2D "/Game/Audio/SFX/Stage2/SFX_DoorOpen2.SFX_DoorOpen2" 1.0 1.0 0.0 0 0)))))

(event OnComponentBeginOverlap(Box)
  (params (OverlappedComponent :type Primitive%20Component%20Object%20Reference) (OtherActor :type Actor%20Object%20Reference) (OtherComp :type Primitive%20Component%20Object%20Reference) (OtherBodyIndex :type Integer) (bFromSweep :type Boolean) (SweepResult :type Hit%20Result%20Structure%20%28by%20ref%29))
  (bind _asfrcharacter_base (Utilities|Casting|CastToFRCharacterBase OtherActor))
  (Utilities|FlowControl|DoOnce false
    (:Completed
      (Input|DisableInput _asfrcharacter_base (Game|GetPlayerController 0))
      (bind _outactor (Sequencer|Player|CreateLevelSequencePlayer "/Game/Cinematic/Stage1_ButtonZoomin.Stage1_ButtonZoomin"))
      (Sequencer|Player|Play (Variables|/Script/LevelSequence.LevelSequenceActor|GetSequencePlayer _outactor) :!class /Script/MovieScene.MovieSceneSequencePlayer)
      (Utilities|FlowControl|Delay 2.5)
      (Transformation|SetActorLocation "-112.000000,-2014.000000,284.000000" false false)
      (Input|EnableInput (Game|GetPlayerCharacter 0) (Game|GetPlayerController 0))
      (Utilities|FlowControl|Delay 0.5)
      (bind _returnvalue (Actor|GetActorOfClass "/Game/Blueprints/Stage1/BP_Stage1_4.BP_Stage1_4_C"))
      ;[1 1 1] DialogueActor를 디테일창에서 할당해 재활용
      (bind _asfrcharacter_base_2 (Utilities|Casting|CastToFRCharacterBase (Game|GetPlayerCharacter 0)))
      (bind _output_get (Variables|/Script/FinalRequital.FRCharacterBase|SetInteractiveActor _asfrcharacter_base_2 _returnvalue))
      (Class|FRInteractableBase|Interact _output_get))))

(event Custom|ActivateRotatingDoor
  (bind _floattrack (Timeline|Timeline Play)
    (:Update
      (Transformation|SetRelativeRotation (Variables|Default|GetSM_Door) (Math|Rotator|Lerp(Rotator) "0.000000,-90.000000,0.000000" "0.000000,20.000000,0.000000" _floattrack) false false))))

(event EventBeginPlay)

(fn ConstructionScript)