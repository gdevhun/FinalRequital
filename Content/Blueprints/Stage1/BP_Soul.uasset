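; BP_Soul is a Stage 1 trigger actor that plays a one-time mid-stage event when the player character overlaps its sphere.
; The event fades the screen, disables input and plays the Stage1_Trigger level sequence, with a delayed camera shake during playback.
; Timed delays, rather than sequence callbacks, then restore input, repeat the fade and destroy BP_InvisibleWall and all MidEventLocker-tagged actors to open progression.
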(event OnComponentBeginOverlap(Sphere)
  (params (OverlappedComponent :type Primitive%20Component%20Object%20Reference) (OtherActor :type Actor%20Object%20Reference) (OtherComp :type Primitive%20Component%20Object%20Reference) (OtherBodyIndex :type Integer) (bFromSweep :type Boolean) (SweepResult :type Hit%20Result%20Structure%20%28by%20ref%29))
  (if (Class|GameplayStatics|ObjectIsA OtherActor "/Script/FinalRequital.FRGASCharacterPlayer")
    (Utilities|FlowControl|DoOnce false
      (:Completed
        (CallFunction|PlayLevelSequence)))))

(event Custom|PlayLevelSequence
  (bind _fadewidget (Variables|Default|GetFadeWidget))
  (bind _fadewidget_2 (Variables|Default|GetFadeWidget))
  (UserInterface|Viewport|AddtoViewport _fadewidget 0)
  (Default|PlayFadeOut _fadewidget)
  (Input|DisableInput (Game|GetPlayerCharacter 0) (Game|GetPlayerController 0))
  (bind _outactor (Sequencer|Player|CreateLevelSequencePlayer "/Game/Cinematic/Stage1_Trigger.Stage1_Trigger"))
  (Sequencer|Player|Play (Variables|/Script/LevelSequence.LevelSequenceActor|GetSequencePlayer _outactor) :!class /Script/MovieScene.MovieSceneSequencePlayer)
  (Utilities|FlowControl|Delay 3.0)
  (bind _returnvalue (CameraShakes|StartCameraShake (Game|GetPlayerCameraManager 0) "/Game/Blueprints/Stage1/BP_CameraShake_Stage1.BP_CameraShake_Stage1_C" 2.0 "CameraLocal" "0, 0, 0"))
  (Utilities|FlowControl|Delay 3.5)
  (CameraShakes|StopCameraShake (Game|GetPlayerCameraManager 0) _returnvalue false)
  (Utilities|FlowControl|Delay 2.5)
  (Input|EnableInput (Game|GetPlayerCharacter 0) (Game|GetPlayerController 0))
  (UserInterface|Viewport|AddtoViewport _fadewidget_2 0)
  (Default|PlayFadeOut _fadewidget_2)
  (bind _returnvalue_2 (Actor|GetActorOfClass "/Game/Blueprints/Stage1/BP_InvisibleWall.BP_InvisibleWall_C"))
  (Actor|DestroyActor _returnvalue_2)
  (bind _outactors (Actor|GetAllActorswithTag "MidEventLocker"))
  (for _array_element _outactors
    (Actor|DestroyActor _array_element)))

(fn ConstructionScript)