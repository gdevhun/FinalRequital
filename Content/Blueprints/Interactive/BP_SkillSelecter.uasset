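; BP_SkillSelecter is an interactable that opens a skill selection UI.
; Interact adds SkillSelectWidget to the viewport and hands it to the player controller, provided IsDoOnce is unset and no selection is made.
; Deactivate sets IsDoOnce to block further interaction, hides the interaction prompt and removes the selection UI through the player controller.
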(event Custom|Deactivate
  (Variables|Default|SetbIsDoOnce true)
  (Rendering|SetVisibility (Variables|Default|GetInteractionPromptWidget) false false)
  (Class|FRStackBaseWidget|RemoveUIwithPlayerController (Variables|Default|GetSkillSelectWidget)))

(event EventBeginPlay)

(event EventInteract
  (bind _skillselectwidget (Variables|Default|GetSkillSelectWidget))
  (if (not (Variables|Default|GetbIsDoOnce))
    (if (not (Variables|/Game/UI/WBP_SkillSelect.WBP_SkillSelect_C|GetIsSelected _skillselectwidget))
      (UserInterface|Viewport|AddtoViewport _skillselectwidget 0)
      (Class|FRStackBaseWidget|AddUIwithPlayerController _skillselectwidget _skillselectwidget))))

(fn ConstructionScript)