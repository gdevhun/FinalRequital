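; BP_Stage2ClearException is a Stage 2 actor that reveals a door and clears tagged actors, apparently for stage completion.
; Its SetVisible event enables query and physics collision on the door, unhides it and two other meshes, then destroys every actor tagged "Destroy".
; An unconnected chain would call SetVisible after a delay and play the Stage2_Clear level sequence, but it never runs.
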(event Custom|SetVisible
  (Collision|SetCollisionEnabled (Variables|Default|GetSM_Door) "QueryAndPhysics")
  (Development|SetHiddeninGame (Variables|Default|GetSM_Door) false false)
  (bind _outactors (Actor|GetAllActorswithTag "Destroy"))
  (for _array_element _outactors
    (Actor|DestroyActor _array_element)))

(event EventBeginPlay)

(fn ConstructionScript)