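; BP_Computer is an interactable Stage 2 computer that toggles between the player camera and an inspect view of its monitor.
; Interact asks FRPlayerController to switch to the inspect camera, plays a turn-on sound, and steps the monitor material through two timed changes.
; Interacting again returns to the player camera and resets the material.
; An IsProcessing flag blocks further input during the timed boot sequence.
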(event EventBeginPlay
  (Variables|Default|SetIsInteracting false)
  (Variables|Default|SetIsProcessing false))

(event EventInteract
  (bind _mesh (Variables|Character|GetMesh))
  (if (not (Variables|Default|GetIsProcessing))
    (Variables|Default|SetIsProcessing true)
    (if (Variables|Default|GetIsInteracting)
      (Variables|Default|SetIsInteracting false)
      (bind _asfrplayer_controller (Utilities|Casting|CastToFRPlayerController (Game|GetPlayerController 0)))
      (Class|FRPlayerController|ReturntoPlayerCamera _asfrplayer_controller 0.0)
      (Rendering|Material|SetMaterial (Variables|Character|GetMesh) 0 "/Game/Designer/Material/S2/MI_S2_Monitor_A01.MI_S2_Monitor_A01")
      (Variables|Default|SetIsProcessing false)
      (else
        (Variables|Default|SetIsInteracting true)
        (bind _asfrplayer_controller_2 (Utilities|Casting|CastToFRPlayerController (Game|GetPlayerController 0)))
        (Class|FRPlayerController|SwitchtoInspectCamera _asfrplayer_controller_2 self 0.0 1e+02 0.0)
        (Audio|Components|Audio|Play (Variables|Default|GetAudio_TurnOn) 0.0)
        (Utilities|FlowControl|Delay 1.5)
        (Rendering|Material|SetMaterial _mesh 0 "/Game/Designer/Material/S2/MI_S2_Monitor_A04.MI_S2_Monitor_A04")
        (Utilities|FlowControl|Delay 1.5)
        (Rendering|Material|SetMaterial _mesh 0 "/Game/Designer/Material/S2/MI_S2_Monitor_A03.MI_S2_Monitor_A03")
        (Variables|Default|SetIsProcessing false)))))

(fn ConstructionScript)