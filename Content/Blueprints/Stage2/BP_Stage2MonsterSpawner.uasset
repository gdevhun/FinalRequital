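; BP_Stage2MonsterSpawner is a placed actor that spawns monsters for the Stage 2 gimmick.
; On BeginPlay it finds BP_Stage2GimmickManager and binds to its start and initialize gimmick events.
; On start it spawns each class in MonsterToSpawn at its root transform, applies level effect 2 and tracks the result.
; On initialize it destroys all tracked monsters and clears the array.
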(event Custom|StartGimmick
  (for _array_element (Variables|Default|GetMonsterToSpawn)
    (bind _returnvalue (Game|SpawnActorfromClass _array_element (Transformation|GetWorldTransform (Variables|Default|GetDefaultSceneRoot)) "AdjustIfPossibleButAlwaysSpawn" "MultiplyWithRoot" 0 0))
    (Class|FRMonsterBase|ApplyLevelEffect _returnvalue 2)
    (Utilities|Array|Add (Variables|Default|GetSpanwedMonsterArr) _returnvalue)))

(event Custom|InitializeGimmick
  (for _array_element (Variables|Default|GetSpanwedMonsterArr)
    (Actor|DestroyActor _array_element))
  (Utilities|Array|Clear (Variables|Default|GetSpanwedMonsterArr)))

(event EventBeginPlay
  (bind _returnvalue (Actor|GetActorOfClass "/Game/Blueprints/Stage2/BP_Stage2GimmickManager.BP_Stage2GimmickManager_C"))
  (EventDispatchers|BindEventtoStartGimmick _returnvalue (EventDispatchers|CreateEvent :!event Custom|StartGimmick))
  (EventDispatchers|BindEventtoInitializeGimmick _returnvalue (EventDispatchers|CreateEvent :!event Custom|InitializeGimmick)))

(fn ConstructionScript)