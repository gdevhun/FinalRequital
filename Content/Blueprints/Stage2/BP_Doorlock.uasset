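; BP_Doorlock is an interactable door lock that the player inspects up close and that swings open once unlocked.
; Interact toggles between an inspect camera with a selection widget and the normal player camera, via FRPlayerController.
; UnlockDoor plays a timeline that rotates the mesh open, restores the camera, hides the selection and prompt widgets, and sets IsDoOnce to block further interaction.
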(event Custom|UnlockDoor
  (Utilities|FlowControl|Sequence
    (:then_0
      (Audio|PlaySound2D "/Game/Audio/SFX/Stage2/SFX_DoorOpen2.SFX_DoorOpen2" 1.0 1.0 0.0 0 0)
      (bind _rotatetrack (Timeline|Timeline PlayFromStart)
        (:Update
          (Transformation|SetRelativeRotation (Variables|Character|GetMesh) (Math|Rotator|Lerp(Rotator) "0, 0, 0" "0.000000,100.000000,0.000000" _rotatetrack) false false))))
    (:then_1
      (bind _asfrplayer_controller (Utilities|Casting|CastToFRPlayerController (Game|GetPlayerController 0)))
      (Class|FRPlayerController|ReturntoPlayerCamera _asfrplayer_controller 0.0)
      (Class|FRInteractableObject|HideSelectionWidget)
      (Rendering|SetVisibility (Variables|Default|GetInteractionPromptWidget) false false)
      (Variables|Default|SetbIsDoOnce true))))

(event EventBeginPlay)

(event EventInteract
  (if (not (Variables|Default|GetbIsDoOnce))
    (if (Variables|Default|GetIsInteracting)
      (Variables|Default|SetIsInteracting false)
      (bind _asfrplayer_controller (Utilities|Casting|CastToFRPlayerController (Game|GetPlayerController 0)))
      (Class|FRPlayerController|ReturntoPlayerCamera _asfrplayer_controller 0.0)
      (Class|FRInteractableObject|HideSelectionWidget)
      (else
        (Variables|Default|SetIsInteracting true)
        (bind _asfrplayer_controller_2 (Utilities|Casting|CastToFRPlayerController (Game|GetPlayerController 0)))
        (Class|FRPlayerController|SwitchtoInspectCamera _asfrplayer_controller_2 self 0.0 8e+01 -4e+01)
        (Audio|PlaySound2D "/Game/Audio/SFX/Stage2/SFX_Unlock.SFX_Unlock" 1.0 1.0 0.0 0 0)
        (Class|FRInteractableObject|ShowSelectionWidget)))))

(fn ConstructionScript)