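; BP_LEE_NPC_ClearGimmick is the Stage 2 NPC that clears the stage gimmick when interacted with and leads into a memory video.
; Interact sets BP_Stage2GimmickManager's cleared flag, calls its InitializeGimmickBroadcast, then starts dialogue.
; When dialogue finishes, it disables player input and plays the Stage2_Clear level sequence.
; Timed delays then trigger a WBP_FadeAnim fade-in, followed by BP_Stage2MediaPlayer playback.
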(event EventBeginPlay)

(event EventInteract
  (bind _returnvalue (Actor|GetActorOfClass "/Game/Blueprints/Stage2/BP_Stage2GimmickManager.BP_Stage2GimmickManager_C"))
  (Variables|/Game/Blueprints/Stage2/BP_Stage2GimmickManager.BP_Stage2GimmickManager_C|SetIsGimmickCleared _returnvalue true)
  (Default|InitializeGimmickBroadcast _returnvalue)
  (Class|FRDialogueActor|StartDialogue))

(event EventDialogueFinishCallback
  ;[1 1 1] 시퀀스 후 기억영상
  (Input|DisableInput (Game|Player|GetPlayerPawn 0) (Game|GetPlayerController 0))
  (bind _outactor (Sequencer|Player|CreateLevelSequencePlayer "/Game/Cinematic/Stage2_Clear.Stage2_Clear"))
  (Sequencer|Player|Play (Variables|/Script/LevelSequence.LevelSequenceActor|GetSequencePlayer _outactor) :!class /Script/MovieScene.MovieSceneSequencePlayer)
  (Utilities|FlowControl|Delay 5.0)
  (bind _returnvalue (UserInterface|CreateWidget "/Game/UI/WBP_FadeAnim.WBP_FadeAnim_C"))
  (UserInterface|Viewport|AddtoViewport _returnvalue 0)
  (Default|PlayFadein _returnvalue)
  (Utilities|FlowControl|Delay 2.0)
  (bind _returnvalue_2 (Actor|GetActorOfClass "/Game/Blueprints/ETC/BP_Stage2MediaPlayer.BP_Stage2MediaPlayer_C"))
  (Default|PlayMediaPlayer _returnvalue_2))

(fn ConstructionScript)