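; BP_Stage2AudioPlayer is a Stage 2 audio player that plays and stops gimmick audio through its Audio component.
; On BeginPlay it finds BP_Stage2GimmickManager and binds events to that manager's initialize-gimmick and start-gimmick notifications.
; PlayGimmickAudio plays the sound from the beginning, and StopGimmickAudio stops it.
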(event Custom|PlayGimmickAudio
  (Audio|Components|Audio|Play (Variables|Default|GetAudio) 0.0))

(event Custom|StopGimmickAudio
  (if (Audio|Components|Audio|IsPlaying (Variables|Default|GetAudio))
    _
    (else
      _))
  (Audio|Components|Audio|Stop (Variables|Default|GetAudio)))

(event EventBeginPlay
  (bind _returnvalue (Actor|GetActorOfClass "/Game/Blueprints/Stage2/BP_Stage2GimmickManager.BP_Stage2GimmickManager_C"))
  (EventDispatchers|BindEventtoInitializeGimmick _returnvalue (EventDispatchers|CreateEvent :!event Custom|StopGimmickAudio))
  (EventDispatchers|BindEventtoStartGimmick _returnvalue (EventDispatchers|CreateEvent :!event Custom|PlayGimmickAudio)))

(fn ConstructionScript)