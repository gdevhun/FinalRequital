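; BP_Stage2GimmickManager runs the Stage 2 ordered gimmick puzzle, broadcasting its start and reset.
; Start fires CallStartGimmick and shows the stage timer, while initialize fires CallInitializeGimmick, clears progress and shows the fail UI.
; CheckGimmickOrder appends each element and compares the sequence to a pre-built correct array for that step.
; CheckGimmickOrderClear confirms all five match; a delayed start/reset chain in EventGraph is unconnected.
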(event Custom|StartGimmickBroadcast
  (Default|CallStartGimmick)
  (UserInterface|Viewport|AddtoViewport (Variables|Default|GetStageTimerWidget) 0)
  (Variables|Default|SetIsGimmickStarted true))

(event Custom|InitializeGimmickBroadcast
  (Default|CallInitializeGimmick)
  (Variables|Default|SetGimmickOrderNumber 0)
  (Utilities|Array|Clear (Variables|Default|GetCurrentGimmickOrder))
  (Variables|Default|SetIsGimmickStarted false)
  (UserInterface|Viewport|AddtoViewport (Variables|Default|GetGimmickFailUI) 0))

(event EventBeginPlay)

(fn ConstructionScript)

(fn CheckGimmickOrder
  (params (GimmickElem :type E_GimmickOrder%20Enum :default "NewEnumerator0"))
  (Math|Integer|IncrementInt (Variables|Default|GetGimmickOrderNumber)
    (:%20%20
      (Utilities|Array|Add (Variables|Default|GetCurrentGimmickOrder) GimmickElem)
      (switch int (Variables|Default|GetGimmickOrderNumber)
        (:1
          (return (Utilities|Array|Identical (Variables|Default|GetCurrentGimmickOrder) (Variables|Gimmick|GetCorrectGimmickOrder_1))))
        (:2
          (return (Utilities|Array|Identical (Variables|Default|GetCurrentGimmickOrder) (Variables|Gimmick|GetCorrectGimmickOrder_2))))
        (:3
          (return (Utilities|Array|Identical (Variables|Default|GetCurrentGimmickOrder) (Variables|Gimmick|GetCorrectGimmickOrder_3))))
        (:4
          (return (Utilities|Array|Identical (Variables|Default|GetCurrentGimmickOrder) (Variables|Gimmick|GetCorrectGimmickOrder_4))))
        (:5
          (return (Utilities|Array|Identical (Variables|Default|GetCurrentGimmickOrder) (Variables|Gimmick|GetCorrectGimmickOrder_5))))))))

(fn CheckGimmickOrderClear
  (return (and (Utilities|Array|Identical (Variables|Default|GetCurrentGimmickOrder) (Variables|Gimmick|GetCorrectGimmickOrder_5)) (== (Variables|Default|GetGimmickOrderNumber) 5))))