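; Stage 2 LEE NPC that gives dialogue and acts as the checkpoint for the stage's order-based gimmick.
; On interact it starts its own dialogue if the gimmick manager reports the gimmick has not started, otherwise it checks the order.
; A correct order destroys this actor and hands the player's InteractiveActor and dialogue to BP_LEE_NPC_ClearGimmick.
; A wrong order makes the manager broadcast a gimmick initialization.
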(event EventInteract
  (|CallParentFunction)
  (bind _returnvalue (Actor|GetActorOfClass "/Game/Blueprints/Stage2/BP_Stage2GimmickManager.BP_Stage2GimmickManager_C"))
  (if (Variables|/Game/Blueprints/Stage2/BP_Stage2GimmickManager.BP_Stage2GimmickManager_C|GetIsGimmickStarted _returnvalue)
    (bind _returnvalue_2 (Actor|GetActorOfClass "/Game/Blueprints/Stage2/BP_Stage2GimmickManager.BP_Stage2GimmickManager_C"))
    (if (Variables|/Game/Blueprints/Stage2/BP_Stage2GimmickManager.BP_Stage2GimmickManager_C|GetIsGimmickStarted _returnvalue_2)
      (bind _isclear_ (Default|CheckGimmickOrderClear _returnvalue_2))
      (if _isclear_
        (Actor|DestroyActor)
        (bind _asfrcharacter_base (Utilities|Casting|CastToFRCharacterBase (Game|Player|GetPlayerPawn 0)))
        (bind _returnvalue_3 (Actor|GetActorOfClass "/Game/Blueprints/Stage2/BP_LEE_NPC_ClearGimmick.BP_LEE_NPC_ClearGimmick_C"))
        (Variables|/Script/FinalRequital.FRCharacterBase|SetInteractiveActor _asfrcharacter_base _returnvalue_3)
        (Class|FRDialogueActor|StartDialogue _returnvalue_3)
        (Actor|DestroyActor)
        (else
          (Default|InitializeGimmickBroadcast _returnvalue_2))))
    (else
      (Class|FRDialogueActor|StartDialogue))))

(event EventDialogueFinishCallback)

(fn ConstructionScript)