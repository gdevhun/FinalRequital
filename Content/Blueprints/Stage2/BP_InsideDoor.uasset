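; BP_InsideDoor is an interactable Stage 2 door that swings open a single time.
; Interact passes through a DoOnce, then starts the rotation, sets the IsDoOnce flag, hides the interaction prompt and plays the door-open sound in 2D.
; A Timeline track drives a yaw lerp from StartYaw to EndYaw on the mesh's relative rotation, without sweep.
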(event Custom|ActivateRotatingDoor
  (bind _rotatetrack (Timeline|Timeline PlayFromStart)
    (:Update
      (Transformation|SetRelativeRotation (Variables|Character|GetMesh) (Math|Rotator|Lerp(Rotator) (Math|Rotator|MakeRotator 0.0 0.0 (Variables|Setting|GetStartYaw)) (Math|Rotator|MakeRotator 0.0 0.0 (Variables|Setting|GetEndYaw)) _rotatetrack) false false))))

(event EventBeginPlay)

(event EventInteract
  (Utilities|FlowControl|DoOnce false
    (:Completed
      (CallFunction|ActivateRotatingDoor)
      (Variables|Default|SetbIsDoOnce true)
      (Rendering|SetVisibility (Variables|Default|GetInteractionPromptWidget) false false)
      (Audio|PlaySound2D "/Game/Audio/SFX/Stage2/SFX_DoorOpen.SFX_DoorOpen" 1.0 1.0 0.0 0 0))))

(fn ConstructionScript)