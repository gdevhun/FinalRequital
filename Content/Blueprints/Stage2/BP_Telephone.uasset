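; BP_Telephone is an interactable telephone in Stage 2 that toggles a close-up inspect view with a selection widget.
; Interact switches the FRPlayerController to an inspect camera, plays a sound and shows the widget, or returns to the player camera and hides it.
; An IsProcessing flag guards against re-entry during the toggle.
; On BeginPlay it binds an event to the Stage 2 gimmick manager's gimmick initialization.
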(event EventBeginPlay
  (bind _returnvalue (Actor|GetActorOfClass "/Game/Blueprints/Stage2/BP_Stage2GimmickManager.BP_Stage2GimmickManager_C"))
  (EventDispatchers|BindEventtoInitializeGimmick _returnvalue (EventDispatchers|CreateEvent :!event RestartInteractionSound)))

(event EventInteract
  (if (not (Variables|Default|GetIsProcessing))
    (Variables|Default|SetIsProcessing true)
    (if (Variables|Default|GetIsInteracting)
      (Variables|Default|SetIsInteracting false)
      (bind _asfrplayer_controller (Utilities|Casting|CastToFRPlayerController (Game|GetPlayerController 0)))
      (Class|FRPlayerController|ReturntoPlayerCamera _asfrplayer_controller 0.0)
      (Class|FRInteractableObject|HideSelectionWidget)
      (else
        (Variables|Default|SetIsInteracting true)
        (bind _asfrplayer_controller_2 (Utilities|Casting|CastToFRPlayerController (Game|GetPlayerController 0)))
        (Class|FRPlayerController|SwitchtoInspectCamera _asfrplayer_controller_2 self 0.0 8e+01 0.0)
        (Audio|PlaySound2D "/Game/Audio/SFX/Stage2/SFX_Unlock.SFX_Unlock" 1.0 1.0 0.0 0 0)
        (Class|FRInteractableObject|ShowSelectionWidget)))
    (Variables|Default|SetIsProcessing false)))

(fn ConstructionScript)