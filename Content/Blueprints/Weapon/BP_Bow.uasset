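; BP_Bow is a bow weapon Blueprint that controls the visibility of its nocked arrow mesh.
; The arrow is hidden on BeginPlay and shown through the SpawnArrowMesh event.
; An ArrowDrawTimeline is set up to slide the arrow back along X and hide it when finished, but nothing in the graph triggers it.
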(event Custom|SpawnArrowMesh
  (Rendering|SetVisibility (Variables|Default|GetArrowMesh) true false))

(event EventBeginPlay
  (Rendering|SetVisibility (Variables|Default|GetArrowMesh) false false))

(event EventTick
  (params (DeltaSeconds :type Float%20%28single-precision%29)))

(fn ConstructionScript)