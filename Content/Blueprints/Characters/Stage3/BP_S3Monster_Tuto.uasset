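; Stage 3 tutorial monster character, exposing events to set its movement speed and play a scripted destruction effect.
; SetMoveMode sets a fixed max walk speed on the CharacterMovement component.
; SpawnEmitter bursts electric destruction particles at the actor with a 2D crush sound, then repeats the particles at a hard-coded world position after a delay.
; Nothing runs on BeginPlay, and neither event is called within this Blueprint.
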(event Custom|SetMoveMode
  (Variables|/Script/Engine.CharacterMovementComponent|SetMaxWalkSpeed (Variables|Character|GetCharacterMovement) 4e+02))

(event Custom|SpawnEmitter
  ;[1 1 1] 이 함수 부르면 움직임
  (Effects|SpawnEmitteratLocation "/Game/Realistic_Starter_VFX_Pack_Vol2/Particles/Destruction/P_Destruction_Electric.P_Destruction_Electric" (Transformation|GetActorLocation) "0, 0, 0" "1.000000,2.000000,2.000000")
  (Audio|PlaySound2D "/Game/Audio/SFX/Player/SFX_crush.SFX_crush" 1.0 1.0 0.0 0 0)
  (Utilities|FlowControl|Delay 4.0)
  (Effects|SpawnEmitteratLocation "/Game/Realistic_Starter_VFX_Pack_Vol2/Particles/Destruction/P_Destruction_Electric.P_Destruction_Electric" "-6045.431183,946.764020,2740.000000" "0, 0, 0" "2.000000,2.000000,2.000000"))

(event EventBeginPlay
  (|CallParentFunction) ; This node is disabled and will not be called.\nDrag off pins to build functionality.
)

(fn ConstructionScript
  (|CallParentFunction))