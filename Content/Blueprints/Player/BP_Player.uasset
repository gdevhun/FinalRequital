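; BP_Player is the player character Blueprint that sets up input and switches animation layers per weapon stance.
; BeginPlay adds the default Enhanced Input mapping context, caches the ABP_Base anim instance and applies the unarmed stance.
; Stance events for unarmed, melee, bow and bronze bell unlink weapon layers, link their own and set walk speed, slower when armed.
; A ground-distance sphere trace feeding the anim instance is present but disconnected.
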(event Custom|UnlinkAllPriorLayers
  (bind _mesh (Variables|Character|GetMesh))
  ;[1 1 1] Animation Layers Section
  (Class|SkeletalMeshComponent|UnlinkAnimClassLayers _mesh "/Game/Animations/Locomotion/ABP_MeleeLayers.ABP_MeleeLayers_C")
  (Class|SkeletalMeshComponent|UnlinkAnimClassLayers _mesh "/Game/Animations/Locomotion/ABP_BowLayers.ABP_BowLayers_C")
  (Class|SkeletalMeshComponent|UnlinkAnimClassLayers _mesh "/Game/Animations/Locomotion/ABP_BronzeBellLayers.ABP_BronzeBellLayers_C"))

(event EventBeginPlay
  (Utilities|FlowControl|Sequence
    (:then_0
      (bind _asbp_player_controller (Utilities|Casting|CastToBP_PlayerController (Pawn|GetController)))
      (Utilities|IsValid (PlayerController|LocalPlayerSubsystems|GetEnhancedInputLocalPlayerSubsystem _asbp_player_controller)
        (:Is%20Valid
          (Input|AddMappingContext (PlayerController|LocalPlayerSubsystems|GetEnhancedInputLocalPlayerSubsystem _asbp_player_controller) "/Game/Input/IMC_Default.IMC_Default" 0 "(bIgnoreAllPressedKeysUntilRelease=True,bForceImmediately=False,bNotifyUserSettings=False)")
          (bind _asabp_base (Utilities|Casting|CastToABP_Base (Components|SkeletalMesh|GetAnimInstance (Variables|Character|GetMesh))))
          (Variables|Default|SetAnimInstance _asabp_base))))
    (:then_1
      (Class|FRGASCharacterPlayer|AdjustUnarmedLayerAnim))))

(event EventTick
  (params (DeltaSeconds :type Float%20%28single-precision%29)))

(event EventAdjustBowLayerAnim
  ;[1 1 1] Animation Layers Section
  (CallFunction|UnlinkAllPriorLayers)
  (Components|SkeletalMesh|AnimationBlueprintLinking|LinkAnimClassLayers (Variables|Character|GetMesh) "/Game/Animations/Locomotion/ABP_BowLayers.ABP_BowLayers_C")
  (Variables|/Script/Engine.CharacterMovementComponent|SetMaxWalkSpeed (Variables|Character|GetCharacterMovement) 4e+02))

(event EventAdjustBronzeBellLayerAnim
  ;[1 1 1] Animation Layers Section
  (CallFunction|UnlinkAllPriorLayers)
  (Components|SkeletalMesh|AnimationBlueprintLinking|LinkAnimClassLayers (Variables|Character|GetMesh) "/Game/Animations/Locomotion/ABP_BronzeBellLayers.ABP_BronzeBellLayers_C")
  (Variables|/Script/Engine.CharacterMovementComponent|SetMaxWalkSpeed (Variables|Character|GetCharacterMovement) 4e+02))

(event EventAdjustMeleeLayerAnim
  ;[1 1 1] Animation Layers Section
  (CallFunction|UnlinkAllPriorLayers)
  (Components|SkeletalMesh|AnimationBlueprintLinking|LinkAnimClassLayers (Variables|Character|GetMesh) "/Game/Animations/Locomotion/ABP_MeleeLayers.ABP_MeleeLayers_C")
  (Variables|/Script/Engine.CharacterMovementComponent|SetMaxWalkSpeed (Variables|Character|GetCharacterMovement) 4e+02))

(event EventAdjustUnarmedLayerAnim
  ;[1 1 1] Animation Layers Section
  (CallFunction|UnlinkAllPriorLayers)
  (Components|SkeletalMesh|AnimationBlueprintLinking|LinkAnimClassLayers (Variables|Character|GetMesh) "/Game/Animations/Locomotion/ABP_UnarmedLayers.ABP_UnarmedLayers_C")
  (Variables|/Script/Engine.CharacterMovementComponent|SetMaxWalkSpeed (Variables|Character|GetCharacterMovement) 5.5e+02))

(fn ConstructionScript)