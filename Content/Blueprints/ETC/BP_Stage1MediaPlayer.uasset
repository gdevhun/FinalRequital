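; Stage 1 movie player that shows one of three cutscene videos, chosen by the player character's acquired memory cell count.
; PlayMediaPlayer adds and prepares the movie widget, opens the matching source, and swaps the level audio for the MediaSound output.
; A hardcoded delay per clip, rather than a media end event, triggers the fade-out widget and fades the audio back in.
; BeginPlay is empty, so playback relies on an external call.
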(event Custom|PlayMovieSound
  ;[1 1 1] When Playing Movie, Excute Music Player To Media Sound
  (Media|MediaSoundComponent|SetMediaPlayer (Variables|Default|GetMediaSound) (Variables|Default|GetMediaPlayer))
  (CameraShake|Start (Variables|Default|GetMediaSound))
  (Audio|Components|Audio|Stop (Variables|Default|GetAudio)))

(event Custom|StopMovieSound
  (Media|MediaSoundComponent|SetMediaPlayer (Variables|Default|GetMediaSound) (Variables|Default|GetMediaPlayer))
  (Audio|Components|Audio|Stop (Variables|Default|GetMediaSound))
  (Audio|Components|Audio|FadeIn (Variables|Default|GetAudio) 2.0 1.0 0.0 "Linear" :!class /Script/Engine.AudioComponent))

(event Custom|PlayMediaPlayer
  (bind _mediaplayerwidget (Variables|Default|GetMediaPlayerWidget))
  (bind _fadewidget (Variables|Default|GetFadeWidget))
  (UserInterface|Viewport|AddtoViewport _mediaplayerwidget 0)
  (Default|PrepareMovie _mediaplayerwidget)
  (Utilities|FlowControl|Delay 0.3)
  (bind _asfrcharacter_base (Utilities|Casting|CastToFRCharacterBase (Game|Player|GetPlayerPawn 0)))
  (switch int (Variables|/Script/FinalRequital.FRCharacterBase|GetMemoryCellAcquireNum _asfrcharacter_base)
    (:0
      (Media|MediaPlayer|OpenSource (Variables|Default|GetMediaPlayer) "/Game/Movies/V_st1_A03.V_st1_A03")
      (CallFunction|PlayMovieSound)
      (Utilities|FlowControl|Delay 58.0))
    (:1
      (Media|MediaPlayer|OpenSource (Variables|Default|GetMediaPlayer) "/Game/Movies/V_st1_A02.V_st1_A02")
      (CallFunction|PlayMovieSound)
      (Utilities|FlowControl|Delay 81.0))
    (:2
      (Media|MediaPlayer|OpenSource (Variables|Default|GetMediaPlayer) "/Game/Movies/V_st1_A01.V_st1_A01")
      (CallFunction|PlayMovieSound)
      (Utilities|FlowControl|Delay 112.0)))
  (UserInterface|Viewport|AddtoViewport _fadewidget 0)
  (Default|PlayFadeOut _fadewidget)
  (CallFunction|StopMovieSound))

(event EventBeginPlay)

(fn ConstructionScript)