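; Stage 2 cutscene player that shows one of three movies based on the player character's acquired memory cell count, then travels to the post-Stage 2 level.
; PlayMediaPlayer fades in, shows the movie widget and swaps the Audio component for MediaSound.
; Hard-coded per-movie delays, rather than end-of-media events, trigger shared cleanup that restores input, HUD and audio, fades out, async-loads Samdo_Stage2After and opens it.
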(event Custom|PlayMovieSound
  ;[1 1 1] When Playing Movie, Excute Music Player To Media Sound
  (Media|MediaSoundComponent|SetMediaPlayer (Variables|Default|GetMediaSound) (Variables|Default|GetMediaPlayer))
  (CameraShake|Start (Variables|Default|GetMediaSound))
  (Audio|Components|Audio|Stop (Variables|Default|GetAudio)))

(event Custom|StopMovieSound
  (Media|MediaSoundComponent|SetMediaPlayer (Variables|Default|GetMediaSound) (Variables|Default|GetMediaPlayer))
  (Audio|Components|Audio|Stop (Variables|Default|GetMediaSound))
  (Audio|Components|Audio|Play (Variables|Default|GetAudio) 0.0))

(event Custom|PlayMediaPlayer
  (bind _fadewidget (Variables|Default|GetFadeWidget))
  (bind _fadewidget_2 (Variables|Default|GetFadeWidget))
  (bind _mediaplayerwidget (Variables|Default|GetMediaPlayerWidget))
  (UserInterface|Viewport|AddtoViewport _fadewidget 0)
  (Default|PlayFadein _fadewidget)
  (Utilities|FlowControl|Delay 1.5)
  (UserInterface|Viewport|AddtoViewport _mediaplayerwidget 0)
  (Default|PrepareMovie _mediaplayerwidget)
  (Utilities|FlowControl|Delay 0.3)
  (bind _asfrcharacter_base (Utilities|Casting|CastToFRCharacterBase (Game|Player|GetPlayerPawn 0)))
  (switch int (Variables|/Script/FinalRequital.FRCharacterBase|GetMemoryCellAcquireNum _asfrcharacter_base)
    (:0
      (Media|MediaPlayer|OpenSource (Variables|Default|GetMediaPlayer) "/Game/Movies/V_st2_A03.V_st2_A03")
      (CallFunction|PlayMovieSound)
      (Utilities|FlowControl|Delay 39.0))
    (:1
      (Media|MediaPlayer|OpenSource (Variables|Default|GetMediaPlayer) "/Game/Movies/V_st2_A02.V_st2_A02")
      (CallFunction|PlayMovieSound)
      (Utilities|FlowControl|Delay 53.0))
    (:2
      (Media|MediaPlayer|OpenSource (Variables|Default|GetMediaPlayer) "/Game/Movies/V_st2_A01.V_st2_A01")
      (CallFunction|PlayMovieSound)
      (Utilities|FlowControl|Delay 86.0)))
  (CallFunction|RemoveMovieSet)
  (UserInterface|Viewport|AddtoViewport _fadewidget_2 0)
  (Default|PlayFadeOut _fadewidget_2)
  (CallFunction|StopMovieSound)
  (Utilities|FlowControl|Delay 1.5)
  (bind _object (Utilities|AsyncLoadAsset "/Game/Maps/Samdo/Samdo_Stage2After.Samdo_Stage2After")
    (:Completed
      (Game|OpenLevel(byName) (Utilities|String|StringToName (Utilities|GetDisplayName _object))))))

(event Custom|RemoveMovieSet
  (bind _asfrplayer_controller (Utilities|Casting|CastToFRPlayerController (Game|GetPlayerController 0)))
  (bind _returnvalue (Class|FRPlayerController|GetHUDWidget _asfrplayer_controller))
  (Input|EnableInput (Game|Player|GetPlayerPawn 0) (Game|GetPlayerController 0))
  (Class|FRHUDWidget|SetHUDVisibility _returnvalue true)
  (Widget|RemovefromParent (Variables|Default|GetMediaPlayerWidget)))

(event EventBeginPlay)

(fn ConstructionScript)