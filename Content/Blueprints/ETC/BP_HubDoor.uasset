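; BP_HubDoor is a double door that swings open when the player walks into its trigger box.
; The box overlap calls ActivateRotatingDoor, which starts separate timelines that lerp the relative yaw of the left and right door meshes.
; A DoOnce sits before the FRGASCharacterPlayer check, so the first overlap by any actor uses up the trigger, and the file has no reset or close logic.
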(event OnComponentBeginOverlap(Box)
  (params (OverlappedComponent :type Primitive%20Component%20Object%20Reference) (OtherActor :type Actor%20Object%20Reference) (OtherComp :type Primitive%20Component%20Object%20Reference) (OtherBodyIndex :type Integer) (bFromSweep :type Boolean) (SweepResult :type Hit%20Result%20Structure%20%28by%20ref%29))
  (Utilities|FlowControl|DoOnce false
    (:Completed
      (if (Class|GameplayStatics|ObjectIsA OtherActor "/Script/FinalRequital.FRGASCharacterPlayer")
        (CallFunction|ActivateRotatingDoor)))))

(event Custom|ActivateRotatingDoor
  (Utilities|FlowControl|Sequence
    (:then_0
      (bind _rotatetrack (Timeline|TL_LeftDoor PlayFromStart)
        (:Update
          (Transformation|SetRelativeRotation (Variables|Default|GetSM_LeftDoor) (Math|Rotator|Lerp(Rotator) "0.000000,0.000000,0.000000" "0.000000,-40.000000,0.000000" _rotatetrack) false false))))
    (:then_1
      (bind _rotatetrack_2 (Timeline|TL_RightDoor PlayFromStart)
        (:Update
          (Transformation|SetRelativeRotation (Variables|Default|GetSM_RightDoor) (Math|Rotator|Lerp(Rotator) "0.000000,-180.000000,0.000000" "0.000000,-340.000000,0.000000" _rotatetrack_2) false false))))))

(event EventBeginPlay)

(fn ConstructionScript)