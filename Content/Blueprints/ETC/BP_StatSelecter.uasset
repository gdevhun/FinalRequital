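; BP_StatSelecter is a trigger actor that offers the player a stat selection UI.
; When an FRGASCharacterPlayer enters its Box, it creates a WBP_StatSelect widget and, if no stat is marked selected, shows it and calls AddUIWithPlayerController.
; Leaving the Box removes the widget and calls RemoveUIWithPlayerController.
; An IsPlayerNotSelected flag, set on BeginPlay and cleared by the Deactivate event, gates both overlap responses.
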(event OnComponentBeginOverlap(Box)
  (params (OverlappedComponent :type Primitive%20Component%20Object%20Reference) (OtherActor :type Actor%20Object%20Reference) (OtherComp :type Primitive%20Component%20Object%20Reference) (OtherBodyIndex :type Integer) (bFromSweep :type Boolean) (SweepResult :type Hit%20Result%20Structure%20%28by%20ref%29))
  (if (and (Variables|Default|GetIsPlayerNotSelected) (Class|GameplayStatics|ObjectIsA OtherActor "/Script/FinalRequital.FRGASCharacterPlayer"))
    (bind _returnvalue (UserInterface|CreateWidget "/Game/UI/WBP_StatSelect.WBP_StatSelect_C"))
    (if (not (Variables|/Game/UI/WBP_StatSelect.WBP_StatSelect_C|GetbIsSelectedStat _returnvalue))
      (UserInterface|Viewport|AddtoViewport _returnvalue 0)
      (Class|FRStackBaseWidget|AddUIwithPlayerController _returnvalue _returnvalue))))

(event OnComponentEndOverlap(Box)
  (params (OverlappedComponent :type Primitive%20Component%20Object%20Reference) (OtherActor :type Actor%20Object%20Reference) (OtherComp :type Primitive%20Component%20Object%20Reference) (OtherBodyIndex :type Integer))
  (if (and (Variables|Default|GetIsPlayerNotSelected) (Class|GameplayStatics|ObjectIsA OtherActor "/Script/FinalRequital.FRGASCharacterPlayer"))
    (Widget|RemovefromParent (stale OnComponentBeginOverlap(Box) _returnvalue))
    (Class|FRStackBaseWidget|RemoveUIwithPlayerController (stale OnComponentBeginOverlap(Box) _returnvalue))))

(event Custom|Deactivate
  (Variables|Default|SetIsPlayerNotSelected false))

(event EventBeginPlay
  (Variables|Default|SetIsPlayerNotSelected true))

(fn ConstructionScript)