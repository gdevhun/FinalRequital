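; BP_MemoryCell is a memory cell actor that, when attached to the soul, unlocks an extra visual mesh on BP_Soul.
; Its AttachtoSoul event activates a particle effect, plays a whoosh sound and looks up BP_Soul by class.
; MemoryCellNum selects the soul's second mesh for "First" and the third otherwise.
; The cell destroys itself after a short delay.
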(event EventAttachtoSoul
  (Components|Activation|Activate (Variables|Default|GetParticleSystem) false)
  (Audio|PlaySound2D "/Game/Audio/SFX/swordwhoosh.swordwhoosh" 1.0 1.0 0.0 0 0)
  (bind _returnvalue (Actor|GetActorOfClass "/Game/Blueprints/Stage1/BP_Soul.BP_Soul_C"))
  (if (== (Variables|Default|GetMemoryCellNum) "First")
    (Class|FRSoul|ActiveSecondVisualMesh _returnvalue)
    (else
      (Class|FRSoul|ActiveThirdVisualMesh _returnvalue)))
  (Utilities|FlowControl|Delay 4.0)
  (Actor|DestroyActor))

(fn ConstructionScript)