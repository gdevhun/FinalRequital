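; Tutorial cinematic actor that plays a movie through a viewport widget, then hands off to the next dialogue.
; PlayMediaPlayer opens the V_OP_A01 source, routing movie sound through MediaSound while pausing the separate Audio playback.
; A fixed delay, rather than a media-end event, triggers widget removal and a fade-out.
; It then restarts Audio and sets BP_Tutorial_5 as the player character's InteractiveActor and calls Interact.
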(event Custom|PlayMovieSound
  ;[1 1 1] When Playing Movie, Excute Music Player To Media Sound
  (Media|MediaSoundComponent|SetMediaPlayer (Variables|Default|GetMediaSound) (Variables|Default|GetMediaPlayer))
  (CameraShake|Start (Variables|Default|GetMediaSound))
  (Audio|Components|Audio|Stop (Variables|Default|GetAudio)))

(event Custom|StopMovieSound
  (Media|MediaSoundComponent|SetMediaPlayer (Variables|Default|GetMediaSound) (Variables|Default|GetMediaPlayer))
  (Audio|Components|Audio|Stop (Variables|Default|GetMediaSound))
  (Audio|Components|Audio|Play (Variables|Default|GetAudio) 0.0))

(event Custom|PlayMediaPlayer
  (bind _mediaplayerwidget (Variables|Default|GetMediaPlayerWidget))
  (UserInterface|Viewport|AddtoViewport _mediaplayerwidget 0)
  (Default|PrepareMovie _mediaplayerwidget)
  (Utilities|FlowControl|Delay 0.3)
  (Media|MediaPlayer|OpenSource (Variables|Default|GetMediaPlayer) "/Game/Movies/V_OP_A01.V_OP_A01")
  (CallFunction|PlayMovieSound)
  (Utilities|FlowControl|Delay 71.0)
  (Widget|RemovefromParent (Variables|Default|GetMediaPlayerWidget))
  (bind _returnvalue (UserInterface|CreateWidget "/Game/UI/WBP_FadeAnim.WBP_FadeAnim_C"))
  (UserInterface|Viewport|AddtoViewport _returnvalue 0)
  (Default|PlayFadeOut _returnvalue)
  (Utilities|FlowControl|Delay 3.0)
  (CallFunction|StopMovieSound)
  ;[1 1 1] 영상 끝나고 다음 대화 진행 (BP_Tutorial5)
  (bind _asfrcharacter_base (Utilities|Casting|CastToFRCharacterBase (Game|Player|GetPlayerPawn 0)))
  (bind _returnvalue_2 (Actor|GetActorOfClass "/Game/Blueprints/Tutorial/BP_Tutorial_5.BP_Tutorial_5_C"))
  (bind _output_get (Variables|/Script/FinalRequital.FRCharacterBase|SetInteractiveActor _asfrcharacter_base _returnvalue_2))
  (Class|FRInteractableBase|Interact _output_get))

(event EventBeginPlay)

(fn ConstructionScript)