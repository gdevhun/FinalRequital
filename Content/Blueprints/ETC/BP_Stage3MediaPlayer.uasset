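; Stage 3 movie player that shows one of three cutscene videos, chosen by the player character's acquired memory cell count.
; PlayMediaPlayer fades in, shows the movie widget, opens the video and swaps the level audio for MediaSound.
; Fixed per-video delays, rather than media-end events, trigger teardown: restoring HUD and input, fading out and restarting audio.
; It then plays the Stage3_Clear sequence of a rising door.
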(event Custom|PlayMovieSound
  ;[1 1 1] When Playing Movie, Excute Music Player To Media Sound
  (Media|MediaSoundComponent|SetMediaPlayer (Variables|Default|GetMediaSound) (Variables|Default|GetMediaPlayer))
  (CameraShake|Start (Variables|Default|GetMediaSound))
  (Audio|Components|Audio|Stop (Variables|Default|GetAudio)))

(event Custom|StopMovieSound
  (Media|MediaSoundComponent|SetMediaPlayer (Variables|Default|GetMediaSound) (Variables|Default|GetMediaPlayer))
  (Audio|Components|Audio|Stop (Variables|Default|GetMediaSound))
  (Audio|Components|Audio|Play (Variables|Default|GetAudio) 0.0))

(event Custom|PlayMediaPlayer
  (bind _fadewidget (Variables|Default|GetFadeWidget))
  (bind _fadewidget_2 (Variables|Default|GetFadeWidget))
  (bind _mediaplayerwidget (Variables|Default|GetMediaPlayerWidget))
  (UserInterface|Viewport|AddtoViewport _fadewidget 0)
  (Default|PlayFadein _fadewidget)
  (Utilities|FlowControl|Delay 1.5)
  (UserInterface|Viewport|AddtoViewport _mediaplayerwidget 0)
  (Default|PrepareMovie _mediaplayerwidget)
  (Utilities|FlowControl|Delay 0.3)
  (bind _asfrcharacter_base (Utilities|Casting|CastToFRCharacterBase (Game|Player|GetPlayerPawn 0)))
  (switch int (Variables|/Script/FinalRequital.FRCharacterBase|GetMemoryCellAcquireNum _asfrcharacter_base)
    (:0
      (Media|MediaPlayer|OpenSource (Variables|Default|GetMediaPlayer) "/Game/Movies/V_st3_A03.V_st3_A03")
      (CallFunction|PlayMovieSound)
      (Utilities|FlowControl|Delay 61.0))
    (:1
      (Media|MediaPlayer|OpenSource (Variables|Default|GetMediaPlayer) "/Game/Movies/V_st3_A02.V_st3_A02")
      (CallFunction|PlayMovieSound)
      (Utilities|FlowControl|Delay 114.0))
    (:2
      (Media|MediaPlayer|OpenSource (Variables|Default|GetMediaPlayer) "/Game/Movies/V_st3_A01.V_st3_A01")
      (CallFunction|PlayMovieSound)
      (Utilities|FlowControl|Delay 176.0)))
  (CallFunction|RemoveMovieSet)
  (UserInterface|Viewport|AddtoViewport _fadewidget_2 0)
  (Default|PlayFadeOut _fadewidget_2)
  (CallFunction|StopMovieSound)
  ;[1 1 1] 문올라오는 시퀀스재생
  (bind _outactor (Sequencer|Player|CreateLevelSequencePlayer "/Game/Cinematic/Stage3_Clear.Stage3_Clear"))
  (Sequencer|Player|Play (Variables|/Script/LevelSequence.LevelSequenceActor|GetSequencePlayer _outactor) :!class /Script/MovieScene.MovieSceneSequencePlayer))

(event Custom|RemoveMovieSet
  (bind _asfrplayer_controller (Utilities|Casting|CastToFRPlayerController (Game|GetPlayerController 0)))
  (bind _returnvalue (Class|FRPlayerController|GetHUDWidget _asfrplayer_controller))
  (Variables|/Script/FinalRequital.FRPlayerController|SetbIsInteracting _asfrplayer_controller false)
  (Input|EnableInput (Game|Player|GetPlayerPawn 0) 0)
  (Class|FRHUDWidget|SetHUDVisibility _returnvalue true)
  (Widget|RemovefromParent (Variables|Default|GetMediaPlayerWidget))
  (bind _returnvalue_2 (UserInterface|CreateWidget "/Game/UI/WBP_FadeAnim.WBP_FadeAnim_C"))
  (UserInterface|Viewport|AddtoViewport _returnvalue_2 0)
  (Default|PlayFadeOut _returnvalue_2))

(event EventBeginPlay)

(fn ConstructionScript)