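; BP_StageEnterance is a stage entrance with double doors that swing open when a player character walks into its trigger box.
; The box overlap calls ActivateRotatingDoor, which plays a wooden door sound and runs two timelines that lerp the left and right door rotations in opposite directions.
; A DoOnce ahead of the FRGASCharacterPlayer class check limits it to the first overlap, so a non-player actor arriving first uses up the trigger.
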(event OnComponentBeginOverlap(Box)
  (params (OverlappedComponent :type Primitive%20Component%20Object%20Reference) (OtherActor :type Actor%20Object%20Reference) (OtherComp :type Primitive%20Component%20Object%20Reference) (OtherBodyIndex :type Integer) (bFromSweep :type Boolean) (SweepResult :type Hit%20Result%20Structure%20%28by%20ref%29))
  (Utilities|FlowControl|DoOnce false
    (:Completed
      (if (Class|GameplayStatics|ObjectIsA OtherActor "/Script/FinalRequital.FRGASCharacterPlayer")
        (CallFunction|ActivateRotatingDoor)))))

(event Custom|ActivateRotatingDoor
  (Audio|PlaySound2D "/Game/Audio/SFX/Cinematic/SFX_WoodDoor.SFX_WoodDoor" 1.0 1.0 0.0 0 0)
  (Utilities|FlowControl|Sequence
    (:then_0
      (bind _rotatetrack (Timeline|TL_LeftDoor PlayFromStart)
        (:Update
          (Transformation|SetRelativeRotation (Variables|Default|GetSM_LeftDoor) (Math|Rotator|Lerp(Rotator) "0.000000,-180.000000,0.000000" "0.000000,-70.000000,0.000000" _rotatetrack true) false false))))
    (:then_1
      (bind _rotatetrack_2 (Timeline|TL_RightDoor PlayFromStart)
        (:Update
          (Transformation|SetRelativeRotation (Variables|Default|GetSM_RightDoor) (Math|Rotator|Lerp(Rotator) "0.000000,-180.000000,0.000000" "0.000000,70.000000,0.000000" _rotatetrack_2 true) false false))))))

(event EventBeginPlay)

(fn ConstructionScript)