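; Fire soul stick Blueprint with three braziers that light up to mark stage-clear progress.
; Each brazier pairs an activatable fire component with three components that start hidden.
; BeginPlay restores earlier fires from StageCleared, where 2 lights the first brazier and 3 the first two.
; Three callable events light individual braziers by activating the fire and revealing its components.
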(event Custom|ActiveStage3ClearFire
  ;[1 1 1] 이 함수 호출시 3번 화로에 불 붙음
  (Components|Activation|Activate (Variables|Default|GetStage3Clear) true)
  (Development|SetHiddeninGame (Variables|Default|GetSM_S3_1) false false))

(event Custom|ActiveStage1ClearFire
  ;[1 1 1] 이 함수 호출시 1번 화로에 불 붙음
  (Components|Activation|Activate (Variables|Default|GetStage1Clear) true)
  (Development|SetHiddeninGame (Variables|Default|GetSM_S1_1) false false))

(event Custom|ActiveStage2ClearFire
  ;[1 1 1] 이 함수 호출시 2번 화로에 불 붙음
  (Components|Activation|Activate (Variables|Default|GetStage2Clear) true)
  (Development|SetHiddeninGame (Variables|Default|GetSM_S2_1) false false))

(event EventBeginPlay
  (Development|SetHiddeninGame (Variables|Default|GetSM_S1_1) true false)
  (switch name (Variables|Default|GetStageCleared)
    (:2
      (Development|SetHiddeninGame (Variables|Default|GetSM_S1_1) false false)
      (Components|Activation|Activate (Variables|Default|GetStage1Clear) true))
    (:3
      (Development|SetHiddeninGame (Variables|Default|GetSM_S1_1) false false)
      (Components|Activation|Activate (Variables|Default|GetStage1Clear) true))))

(fn ConstructionScript)